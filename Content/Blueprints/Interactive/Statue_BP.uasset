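; Interactive statue that accepts a gem of a matching type.
; When an actor tagged Gem overlaps the trigger, it casts to Gem_BP and compares the gem's type with the statue's Type.
; A match disables the gem's movement, snaps it to the trigger's location with zero rotation and prints the type; a mismatch only prints a debug rejection.
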(event OnComponentBeginOverlap(GemColliderTrigger)
  (params (OverlappedComponent :type Primitive%20Component%20Object%20Reference) (OtherActor :type Actor%20Object%20Reference) (OtherComp :type Primitive%20Component%20Object%20Reference) (OtherBodyIndex :type Integer) (bFromSweep :type Boolean) (SweepResult :type Hit%20Result%20Structure%20%28by%20ref%29))
  ;[1 1 1] Gem Collision
  (if (Actor|ActorHasTag OtherActor "Gem")
    (bind _asgem_bp (Utilities|Casting|CastToGem_BP OtherActor))
    (bind _returnvalue (Class|Gem|GetGemType _asgem_bp))
    (if (== _returnvalue (Variables|Default|GetType))
      (Default|DisableMovement _asgem_bp)
      (Transformation|SetActorLocation _asgem_bp (Transformation|GetWorldLocation (Variables|Default|GetGemColliderTrigger)) false true)
      (Transformation|SetActorRotation _asgem_bp)
      (Development|PrintString (Utilities|String|EnumtoString (Variables|Default|GetType)))
      (else
        (Development|PrintString "Nope")))))

(fn ConstructionScript)