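; Gem_BP is an interactive gem actor that can be frozen in place or returned to where it began.
; It records its start location on BeginPlay, and ResetPosition teleports it back there without a sweep.
; DisableMovement turns off physics simulation on both the gem mesh and the box component; its node for disabling overlap events is disconnected and never runs.
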(event EventBeginPlay
  ;[1 1 1] Assign Start Location
  (Variables|Default|SetStartLocation (Transformation|GetActorLocation)))

(fn ConstructionScript)

(fn DisableMovement
  (Physics|SetSimulatePhysics (Variables|Default|GetGemMesh) false)
  (Physics|SetSimulatePhysics (Variables|Default|GetBoxComponent) false))

(fn ResetPosition
  (Transformation|SetActorLocation (Variables|Default|GetStartLocation) false true))