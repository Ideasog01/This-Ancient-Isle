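; Interactive trigger actor that shows a text message on screen and pauses gameplay when its box is overlapped.
; BeginPlay creates the MessageDisplay_UW widget; an overlap fills it with the message content, adds it to the viewport and pauses through GameMode_BP.
; The widget receives a back-reference to the actor, whose RemoveMessage removes it and unpauses.
; IsDisplaying is never reset here, blocking repeat displays.
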(event OnComponentBeginOverlap(TriggerBox)
  (params (OverlappedComponent :type Primitive%20Component%20Object%20Reference) (OtherActor :type Actor%20Object%20Reference) (OtherComp :type Primitive%20Component%20Object%20Reference) (OtherBodyIndex :type Integer) (bFromSweep :type Boolean) (SweepResult :type Hit%20Result%20Structure%20%28by%20ref%29))
  ;[1 1 1] Box Trigger
  (if (Math|Boolean|NotEqual(Boolean) (Variables|Default|GetbIsDisplaying) true)
    (CallFunction|DisplayMessage)))

(event EventBeginPlay
  ;[1 1 1] Setup User Widget
  (bind _returnvalue (UserInterface|CreateWidget "/Game/UI/MessageDisplay_UW.MessageDisplay_UW_C"))
  (Variables|Default|SetMessageDisplay_UW _returnvalue))

(fn ConstructionScript)

(fn DisplayMessage
  (bind _messagedisplay_uw (Variables|Default|GetMessageDisplay_UW))
  (bind _returnvalue (Class|MessageDisplay|GetMessageContent))
  (Variables|/Game/UI/MessageDisplay_UW.MessageDisplay_UW_C|SettextContent _messagedisplay_uw _returnvalue)
  (UserInterface|Viewport|AddtoViewport _messagedisplay_uw 0)
  (Variables|Default|SetbIsDisplaying true)
  (bind _asgame_mode_bp (Utilities|Casting|CastToGameMode_BP (Game|GetGameMode)))
  (Default|PauseGameplay _asgame_mode_bp true)
  (Variables|/Game/UI/MessageDisplay_UW.MessageDisplay_UW_C|SetmessageDisplayBP (Variables|Default|GetMessageDisplay_UW) self))

(fn RemoveMessage
  (Widget|RemovefromParent (Variables|Default|GetMessageDisplay_UW))
  (bind _asgame_mode_bp (Utilities|Casting|CastToGameMode_BP (Game|GetGameMode)))
  (Default|PauseGameplay _asgame_mode_bp false))