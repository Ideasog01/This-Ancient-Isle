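; GameMode_BP is the game mode that tracks statue progress and handles pausing gameplay.
; OnStatueActivated increments a counter, calls CallOpenCave when the fourth statue activates, and shows the EndScreen_UW widget with the mouse cursor on the fifth.
; PauseGameplay toggles the cursor and sets DisablePlayer on the Player_BP pawn rather than pausing the world.
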(fn ConstructionScript)

(fn PauseGameplay
  (params (bPauseGameplay :type Boolean))
  (Variables|/Script/Engine.PlayerController|SetbShowMouseCursor (Game|GetPlayerController 0) bPauseGameplay)
  (bind _asplayer_bp (Utilities|Casting|CastToPlayer_BP (Game|Player|GetPlayerPawn 0)))
  (Variables|/Script/AncientIsle.PlayerCharacter|SetbDisablePlayer _asplayer_bp bPauseGameplay))

(fn OnStatueActivated
  (bind _returnvalue (Game|GetPlayerController 0))
  (bind _result (Math|Integer|IncrementInt (Variables|Default|GetStatuesActivated))
    (:%20%20
      (Development|PrintString "Statues Activated Incremented.")
      (Variables|Default|SetStatuesActivated _result)
      (Utilities|FlowControl|Sequence
        (:then_0
          ;[1 1 1] Final Statue
          (if (== (Variables|Default|GetStatuesActivated) 5)
            (bind _returnvalue_2 (UserInterface|CreateWidget "/Game/UI/EndScreen_UW.EndScreen_UW_C" _returnvalue))
            (UserInterface|Viewport|AddtoViewport _returnvalue_2 0)
            (Variables|/Script/Engine.PlayerController|SetbShowMouseCursor _returnvalue true)))
        (:then_1
          (if (== (Variables|Default|GetStatuesActivated) 4)
            (Default|CallOpenCave)))))))