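; Player Blueprint that shows the player HUD and provides a camera-based forward point.
; On BeginPlay it creates a PlayerHUD_UW widget for the first player controller and adds it to the viewport.
; Its GetForwardVector function returns a world location ForwardDistance ahead of PlayerCamera along the camera's facing, rather than a direction vector as the name suggests.
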(event EventBeginPlay
  ;[1 1 1] Add Player HUD to Viewport
  (bind _returnvalue (Game|ConstructObjectfromClass "/Game/UI/PlayerHUD_UW.PlayerHUD_UW_C" (Game|GetPlayerController 0)))
  (UserInterface|Viewport|AddtoViewport _returnvalue 0))

(fn ConstructionScript)

(fn GetForwardVector
  (bind _playercamera (Variables|Default|GetPlayerCamera))
  (return (+ (Transformation|GetWorldLocation _playercamera) (* (Math|Vector|GetForwardVector (Transformation|GetWorldRotation _playercamera)) (Variables|Default|GetForwardDistance)))))